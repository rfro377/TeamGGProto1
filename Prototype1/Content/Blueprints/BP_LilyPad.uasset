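; BP_LilyPad is a lily pad actor that, while IsMoving is set, shuttles back and forth between Start and End points.
; Tick advances a clamped alpha by delta time over TripTime and linearly interpolates the root component's relative location, without sweeping.
; When the alpha reaches one, it resets to zero and swaps the endpoints, so the motion repeats in reverse.
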(event `self.ReceiveTick`
  (params (DeltaSeconds :type "Float (single-precision)"))
  (if (`self.isMoving?`)
    (bind _output_get (set `self.Lerpvalue` (`KismetMathLibrary.FClamp` (+ (`self.Lerpvalue`) (/ DeltaSeconds (`self.TripTime`))))))
    (`SceneComponent.K2_SetRelativeLocation` (`self.DefaultSceneRoot`) (`KismetMathLibrary.VLerp` (`self.Start`) (`self.End`) _output_get) false false)
    (if (== (`self.Lerpvalue`) 1.0)
      (set `self.Lerpvalue` 0.0)
      (set `self.Temp` (`self.Start`))
      (set `self.Start` (`self.End`))
      (set `self.End` (`self.Temp`)))))

(fn `UserConstructionScript`)