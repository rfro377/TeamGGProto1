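; BP_PowerFocalPoint_Plant is a power focal point that relays an ability trigger to the targets it affects.
; TriggerEvent checks the trigger ability, then loops through AffectedTargets and fires TriggeredEvent on each one implementing the BP_InteractTargets interface.
; For other actors it falls back to messaging the first component found with that interface.
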(event `TriggerEvent`
  (params (TriggerAbility :type "/Game/UI/Abilities Enum" :default "NewEnumerator0"))
  (if (`|EnumEquality` (`self.TriggerAbility`) TriggerAbility)
    (for _array_element (`self.AffectedTargets`)
      (bind _asbp_interact_targets (cast `/Game/Blueprints/BP_InteractTargets` _array_element)
        (:`then`
          (`/Game/Blueprints/BP_InteractTargets.TriggeredEvent` _asbp_interact_targets null))
        (:`CastFailed`
          (bind _asactor (cast `Actor` _array_element))
          (message `/Game/Blueprints/BP_InteractTargets.TriggeredEvent` (`|GetArrayItem` (`self.GetComponentsByInterface` _asactor "/Game/Blueprints/BP_InteractTargets.BP_InteractTargets_C")) null))))))

(fn `UserConstructionScript`)