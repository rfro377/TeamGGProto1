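; Actor component that offsets its owner vertically by a ZMovement amount once triggered.
; BeginPlay caches the owner's start location and a target along Z, and TriggeredEvent switches on the active flag.
; While active, Tick sets the location with VInterpTo from the cached start, which never updates, so the owner stays a frame-time-dependent fraction of the way instead of progressively approaching the target.
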(event `self.ReceiveBeginPlay`
  (bind _output_get (set `self.Start` (`Actor.K2_GetActorLocation` (`self.GetOwner`))))
  (set `self.End` (+ _output_get (`KismetMathLibrary.MakeVector` 0.0 0.0 (`self.Z_Movement`)))))

(event `self.ReceiveTick`
  (params (DeltaSeconds :type "Float (single-precision)"))
  (if (`self.isActive?`)
    (`Actor.K2_SetActorLocation` (`self.GetOwner` self) (`KismetMathLibrary.VInterpTo` (`self.Start`) (`self.End`) DeltaSeconds 10.0) false false)))

(event `/Game/Blueprints/BP_InteractTargets.TriggeredEvent`
  (params (ActorRef :type "Actor Object Reference"))
  (set `self.isActive?` true))