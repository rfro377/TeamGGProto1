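; BP_Critter is a wandering creature that switches from a dirty look to a clean one when triggered by a water attack.
; It roams by chaining AIMoveTo calls to random reachable points around its spawn location, repeating only when a move succeeds.
; TriggeredEvent accepts only BP_WaterAttack, then hides DirtyCritter and shows CleanCritter.
; The RandomXY helper is not called within this Blueprint.
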(event `self.ReceiveBeginPlay`
  (set `self.StartPos` (`self.K2_GetActorLocation`))
  (`self.Roam`))

(event `/Game/Blueprints/BP_InteractTargets.TriggeredEvent`
  (params (ActorRef :type "Actor Object Reference"))
  (cast `/Game/Attack_BP/BP_WaterAttack` ActorRef)
  (`SceneComponent.SetVisibility` (`self.DirtyCritter`) false false)
  (`SceneComponent.SetVisibility` (`self.CleanCritter`) true false))

(event `Roam`
  (`|AIMoveTo` self (`NavigationSystemV1.K2_GetRandomReachablePointInRadius` (`self.StartPos`) (`self.RoamRadius`) null null) null
    (:`OnSuccess`
      (`self.Roam`))))

(fn `randomXY`
  (returns (ReturnValue :type "Float (double-precision)") (ReturnValue2 :type "Float (double-precision)"))
  (return (- (* (`KismetMathLibrary.RandomFloat`) 2.0) 1.0) (- (* (`KismetMathLibrary.RandomFloat`) 2.0) 1.0)))

(fn `UserConstructionScript`)