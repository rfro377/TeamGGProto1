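; BP_VialThrow is a thrown vial projectile that can trigger interactable targets and breaks on contact.
; On BeginPlay, its capsule gets a random angular impulse so the vial tumbles.
; Overlapping a BP_InteractTargets passes the vial to that target's TriggeredEvent, while any other overlap breaks it.
; Capsule hits with another valid actor also call BreakVial, which simply destroys the actor.
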(event `self.ReceiveBeginPlay`
  (`PrimitiveComponent.AddAngularImpulseInDegrees` (`self.Capsule`) (* (`KismetMathLibrary.RandomUnitVector`) 200.0) "None" true))

(event `self.ReceiveActorBeginOverlap`
  (params (OtherActor :type "Actor Object Reference"))
  ; Interactable check
  (bind _asbp_interact_targets (cast `/Game/Blueprints/BP_InteractTargets` OtherActor)
    (:`then`
      (`/Game/Blueprints/BP_InteractTargets.TriggeredEvent` _asbp_interact_targets self))
    (:`CastFailed`
      ; Destroy on collision
      (`self.BreakVial` :!label _label))))

(event `self.Capsule.OnComponentHit`
  (params (HitComponent :type "PrimitiveComponent Object Reference") (OtherActor :type "Actor Object Reference") (OtherComp :type "PrimitiveComponent Object Reference") (NormalImpulse :type "Vector Structure") (Hit :type "HitResult Structure (by ref)"))
  ; Destroy on collision
  (`/Engine/EditorBlueprintResources/StandardMacros.IsValid` OtherActor
    (:`Is Valid`
      (if (!= OtherActor self)
        (goto _label)))))

(event `BreakVial`
  ; Break Vial - destroy projectile
  (`self.K2_DestroyActor`))

(fn `UserConstructionScript`)